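; BP_TimedPlatform is a platform that turns red and destroys itself after it is hit.
; BeginPlay puts a dynamic material instance on the Cube, and any Hit sets a collision flag with no filter on the other actor.
; Once flagged, Tick counts ColorLerp down by delta time, using it as both the white-to-red Tint blend and the timer that destroys the actor at zero.
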(event `self.ReceiveBeginPlay`
  (bind _returnvalue (`KismetMaterialLibrary.CreateDynamicMaterialInstance` "/Game/Materials/M_PlaftormMaterial.M_PlaftormMaterial"))
  (bind _output_get (set `self.MatRef` _returnvalue))
  (`PrimitiveComponent.SetMaterial` (`self.Cube`) 0 _output_get))

(event `self.ReceiveHit`
  (params (MyComp :type "PrimitiveComponent Object Reference") (Other :type "Actor Object Reference") (OtherComp :type "PrimitiveComponent Object Reference") (bSelfMoved :type Boolean) (HitLocation :type "Vector Structure") (HitNormal :type "Vector Structure") (NormalImpulse :type "Vector Structure") (Hit :type "HitResult Structure (by ref)"))
  (set `self.HasCollided` true))

(event `self.ReceiveTick`
  (params (DeltaSeconds :type "Float (single-precision)"))
  (if (`self.HasCollided`)
    (`|ExecutionSequence`
      (:`then_0`
        (`MaterialInstanceDynamic.SetVectorParameterValue` (`self.MatRef`) "Tint" (`KismetMathLibrary.LinearColorLerp` (`KismetMathLibrary.MakeColor` 1.0) (`KismetMathLibrary.MakeColor` 1.0 1.0 1.0) (stale _output_get))))
      (:`then_1`
        (bind _output_get (set `self.ColorLerp` (`KismetMathLibrary.FClamp` (- (`self.ColorLerp`) (`GameplayStatics.GetWorldDeltaSeconds`)) 0.0 (`self.ColorLerp`)))))
      (:`then_2`
        (if (== (`self.ColorLerp`) 0.0)
          (`self.K2_DestroyActor`))))))

(fn `UserConstructionScript`)