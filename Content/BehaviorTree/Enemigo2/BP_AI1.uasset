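; BP_AI1 is an enemy AI that shoots bullets when it sees the pirate player character.
; PawnSensing sets the "hasSeenPlayer?" blackboard key and spawns a BP_Bullet at SpawnPoint whenever CanAttack allows.
; A CanAttack flag and Delay throttle fire using AttackSpeed from the DT_Enemyshoot row loaded on BeginPlay.
; ApplyDamage targets the spawned bullet itself, not the sighted player, with no damage amount set.
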(event `self.PawnSensing.OnSeePawn`
  (params (Pawn :type "Pawn Object Reference"))
  (cast `/Game/ThirdPerson/Blueprints/BP_ThirdPersonCharacterPirate` Pawn)
  (`BlackboardComponent.SetValueAsBool` (`AIBlueprintHelperLibrary.GetBlackboard` (`AIBlueprintHelperLibrary.GetAIController` self)) "hasSeenPlayer?" true)
  (if (`self.CanAttack?`)
    (bind _returnvalue (`|SpawnActorFromClass` "/Game/BehaviorTree/Enemigo2/BP_Bullet.BP_Bullet_C" (`SceneComponent.K2_GetComponentToWorld` (`self.SpawnPoint`)) "Undefined" "MultiplyWithRoot" null null))
    (`GameplayStatics.ApplyDamage` _returnvalue)
    (set `self.CanAttack?` false)
    (`KismetSystemLibrary.Delay` (`.AttackSpeed_4_E0E4A124494F2D029E565BB3B8944234` (break `/Game/BehaviorTree/Enemigo2/EnemyShoot` (stale `self.ReceiveBeginPlay` _returnvalue))))
    (set `self.CanAttack?` true)))

(event `self.ReceiveBeginPlay`
  (bind _returnvalue (`|GetDataTableRow` "/Game/BehaviorTree/Enemigo2/DT_Enemyshoot.DT_Enemyshoot" "Damage+ShootSpeed")))

(fn `UserConstructionScript`)