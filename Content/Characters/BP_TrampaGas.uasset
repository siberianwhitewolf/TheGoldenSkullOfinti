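; BP_TrampaGas is a gas trap that deals periodic damage to the pirate third-person character while it stands inside the trap's box.
; Entering the box stores the character, activates the particle system and starts a looping one-second timer that applies fixed damage to it.
; Leaving the box clears that timer and deactivates the particles.
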(event `AplicarDaño`
  (`GameplayStatics.ApplyDamage` (stale `self.Box.OnComponentBeginOverlap` _asbp_third_person_character) 10.0))

(event `self.Box.OnComponentBeginOverlap`
  (params (OverlappedComponent :type "PrimitiveComponent Object Reference") (OtherActor :type "Actor Object Reference") (OtherComp :type "PrimitiveComponent Object Reference") (OtherBodyIndex :type Integer) (bFromSweep :type Boolean) (SweepResult :type "HitResult Structure (by ref)"))
  (bind _asbp_third_person_character (cast `/Game/ThirdPerson/Blueprints/BP_ThirdPersonCharacterPirate` OtherActor))
  (bind _returnvalue (`KismetSystemLibrary.K2_SetTimerDelegate` (delegate `AplicarDaño`) 1.0 true))
  (`ActorComponent.Activate` (`self.ParticleSystem`) false))

(event `self.Box.OnComponentEndOverlap`
  (params (OverlappedComponent :type "PrimitiveComponent Object Reference") (OtherActor :type "Actor Object Reference") (OtherComp :type "PrimitiveComponent Object Reference") (OtherBodyIndex :type Integer))
  (cast `/Game/ThirdPerson/Blueprints/BP_ThirdPersonCharacterPirate` OtherActor)
  (`KismetSystemLibrary.K2_ClearAndInvalidateTimerHandle` (stale `self.Box.OnComponentBeginOverlap` _returnvalue))
  (`ActorComponent.Deactivate` (`self.ParticleSystem`)))

(fn `UserConstructionScript`)